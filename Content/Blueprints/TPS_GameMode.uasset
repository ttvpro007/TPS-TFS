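; Third-person shooter game mode that tracks score, kill count and combo streaks.
; AddScore counts a kill, raises the combo, records the best combo and adds the base score multiplied by the current combo.
; Tick runs a combo timer that AddScore restarts, resetting the combo once the time limit passes.
; BeginPlay caches the level's SpawnManager, which this graph does not otherwise use.
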(event Custom|Add%20Score
  (params (Score :type Integer))
  ;[1 1 1] Handle AddScore Event
  (Variables|Default|SetBase%20Score Score)
  (Variables|Default|SetCombo%20Timer 0.0 :!pinned true) ; AddScore will Reset ComboTimer to 0
  (Variables|Default|SetHas%20Combo%20Started true)
  (Variables|Default|SetEnemies%20Killed (+ (Variables|Default|GetEnemies%20Killed) 1))
  (bind _output_get (Variables|Default|SetCurrent%20Combo (+ (Variables|Default|GetCurrent%20Combo) 1) :!pinned true)) ; AddScore will increase Combo by 1
  ;[1 1 1] Set Best Combo
  (Variables|Default|SetBest%20Combo (Math|Integer|Max(Integer) _output_get (Variables|Default|GetBest%20Combo)))
  ;[1 1 1] Combo Scoring System
  (Variables|Default|SetCurrent%20Score (+ (* (Math|Integer|Max(Integer) _output_get 1) (Variables|Default|GetBase%20Score)) (Variables|Default|GetCurrent%20Score))))

(event EventBeginPlay
  (bind _returnvalue (Actor|GetActorOfClass "/Game/Blueprints/SpawnManager.SpawnManager_C"))
  (Variables|Default|SetSpawn%20Manager _returnvalue))

(event EventTick
  (params (DeltaSeconds :type Float%20%28single-precision%29))
  ;[1 1 1] If Combo Started ComboTimer += DeltaSeconds
  (if (Variables|Default|GetHas%20Combo%20Started)
    (bind _output_get (Variables|Default|SetCombo%20Timer (+ DeltaSeconds (Variables|Default|GetCombo%20Timer))))
    ;[1 1 1] If ComboTimer > TimeLimiter Reset Variables
    (if (> _output_get (Variables|Default|GetCombo%20Time%20Limiter))
      (Variables|Default|SetCombo%20Timer 0.0)
      (Variables|Default|SetCurrent%20Combo 0)
      (Variables|Default|SetHas%20Combo%20Started false))))

(fn ConstructionScript)