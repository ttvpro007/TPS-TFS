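; Wave spawner that places a new batch of Humanoid_AI enemies at random points inside its SpawnVolume whenever none remain.
; BeginPlay caches existing enemies and binds the spawn event to the OnAllEnemyDestroyed dispatcher.
; Tick fires that dispatcher once per enemy in a wave when the list empties, guarded by HadFinishedSpawning.
; Otherwise Tick prunes null entries, with a timed world rescan clearing the list if no enemies exist.
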(event Custom|Spawn%20Humanoid%20Enemy
  (bind _output_get (Variables|Default|SetRandom%20Point%20In%20Box (Math|Random|RandomPointinBoundingBox (Transformation|GetWorldLocation (Variables|Default|GetDefaultSceneRoot)) (Components|Box|GetScaledBoxExtent (Variables|Default|GetSpawnVolume)))))
  (bind _returnvalue (Game|SpawnActorfromClass "/Game/Blueprints/Humanoid_AI.Humanoid_AI_C" (Math|Transform|MakeTransform _output_get "0, 0, 0" "1,1,1") "AdjustIfPossibleButDontSpawnIfColliding" 0 0))
  (Utilities|Array|Add (Variables|Default|GetHumanoid%20Enemies) _returnvalue))

(event EventBeginPlay
  (bind _outactors (Actor|GetAllActorsOfClass "/Game/Blueprints/Humanoid_AI.Humanoid_AI_C"))
  (Variables|Default|SetHumanoid%20Enemies _outactors)
  (EventDispatchers|BindEventtoOnAllEnemyDestroyed (delegate Custom|Spawn%20Humanoid%20Enemy)))

(event EventTick
  (params (DeltaSeconds :type Float%20%28single-precision%29))
  (Variables|Default|SetCheck%20Enemy%20List%20Timer (+ DeltaSeconds (Variables|Default|GetCheck%20Enemy%20List%20Timer)))
  (if (== (Utilities|Array|Length (Variables|Default|GetHumanoid%20Enemies)) 0)
    (if (Variables|Default|GetHad%20Finished%20Spawning)
      (for _index (range 0 (- (Variables|Default|GetAmount%20Per%20Wave) 1))
        (Variables|Default|SetHad%20Finished%20Spawning false)
        (Default|CallOnAllEnemyDestroyed))
      (Variables|Default|SetHad%20Finished%20Spawning true)
      (Math|Integer|IncrementInt (Variables|Default|GetWave%20Spawned)
        (:%20%20
          (if (> (Variables|Default|GetCheck%20Enemy%20List%20Timer) (Variables|Default|GetCheck%20Enemy%20List%20Interval)) :!label _label
            (CallFunction|TryResetHumanoidEnemyList)
            (Variables|Default|SetCheck%20Enemy%20List%20Timer 0.0)))))
    (else
      (CallFunction|RemoveNullValueinEnemiesArray)
      (goto _label))))

(fn ConstructionScript)

(fn RemoveNullValueinEnemiesArray
  (bind _humanoid_enemies (Variables|Default|GetHumanoid%20Enemies))
  (for _array_element _humanoid_enemies
    (if (== _array_element 0)
      (Utilities|Array|RemoveItem _humanoid_enemies _array_element))))

(fn TryResetHumanoidEnemyList
  (bind _outactors (Actor|GetAllActorsOfClass "/Game/Blueprints/Humanoid_AI.Humanoid_AI_C"))
  (bind _output_get (LocalVariables|SetCurrent%20Numanoid%20Enemies _outactors))
  (if (== (Utilities|Array|Length _output_get) 0)
    (Utilities|Array|Clear (Variables|Default|GetHumanoid%20Enemies))
    (return true)
    (else
      (return false))))