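; Player pawn Blueprint that sets up the player HUD and handles the weapon's zoom aiming state.
; BeginPlay creates the PlayerUI widget and adds it to the viewport.
; Each tick copies the Zoomed flag to the current weapon's zoom mode.
; While zoomed, it also predicts a projectile path from the muzzle socket at a fixed launch speed, shown only through per-frame debug drawing.
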(event EventBeginPlay
  (bind _returnvalue (UserInterface|CreateWidget "/Game/Blueprints/PlayerUI.PlayerUI_C" (Game|GetPlayerController 0)))
  (UserInterface|Viewport|AddtoViewport _returnvalue 0))

(event EventTick
  (params (DeltaSeconds :type Float%20%28single-precision%29))
  (bind _self self)
  (bind _currentweapon (Variables|Default|GetcurrentWeapon _self))
  (bind _muzzlesocketname (Variables|/Script/TPS.TPSWeapon|GetmuzzleSocketName _currentweapon))
  (bind _meshcomp (Variables|/Script/TPS.TPSWeapon|GetmeshComp _currentweapon))
  (if (Variables|Default|GetbZoomed _self)
    (Variables|/Script/TPS.TPSWeapon|SetWeaponZoomMode _currentweapon "ZOOMED")
    (Class|GameplayStatics|BlueprintPredictProjectilePathbyTraceChannel (Transformation|GetSocketLocation _meshcomp _muzzlesocketname) (* (Math|Vector|GetForwardVector (Transformation|GetSocketRotation _meshcomp _muzzlesocketname)) 3e+03) true 0.0 "ECC_Visibility" false 0 "ForOneFrame" 2.0 15.0 1.0)
    (else
      (Variables|/Script/TPS.TPSWeapon|SetWeaponZoomMode _currentweapon "NORMAL"))))

(fn ConstructionScript)