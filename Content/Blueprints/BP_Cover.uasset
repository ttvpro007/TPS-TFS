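; BP_Cover is a cover actor that tells a PlayerPawn which cover trigger volume it is standing in.
; On BeginPlay it binds begin and end overlap handlers to every BoxComponent it owns, so any number of boxes share the same logic.
; Entering a box stores it in the pawn's CoverTriggerVolume; leaving clears that reference only if it still points to the same box.
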(event Custom|OnBeginOverlap
  (params (OverlappedComponent :type Primitive%20Component%20Object%20Reference) (OtherActor :type Actor%20Object%20Reference) (OtherComp :type Primitive%20Component%20Object%20Reference) (OtherBodyIndex :type Integer) (bFromSweep :type Boolean) (SweepResult :type Hit%20Result%20Structure%20%28by%20ref%29))
  (bind _asplayer_pawn (Utilities|Casting|CastToPlayerPawn OtherActor))
  (bind _asbox_collision (Utilities|Casting|CastToBoxComponent OverlappedComponent))
  (Variables|/Script/TPS.TPSCharacter|SetCoverTriggerVolume _asplayer_pawn _asbox_collision))

(event Custom|OnEndOverlap
  (params (OverlappedComponent :type Primitive%20Component%20Object%20Reference) (OtherActor :type Actor%20Object%20Reference) (OtherComp :type Primitive%20Component%20Object%20Reference) (OtherBodyIndex :type Integer))
  (bind _asplayer_pawn (Utilities|Casting|CastToPlayerPawn OtherActor))
  (bind _asbox_collision (Utilities|Casting|CastToBoxComponent OverlappedComponent))
  (if (== (Variables|/Script/TPS.TPSCharacter|GetCoverTriggerVolume _asplayer_pawn) _asbox_collision)
    (Variables|/Script/TPS.TPSCharacter|SetCoverTriggerVolume _asplayer_pawn 0)))

(event EventBeginPlay
  (for _array_element (Actor|GetComponentsByClass "/Script/Engine.BoxComponent")
    (Collision|BindEventtoOnComponentBeginOverlap _array_element (delegate Custom|OnBeginOverlap))
    (Collision|BindEventtoOnComponentEndOverlap _array_element (delegate Custom|OnEndOverlap))))

(event Collision|EventActorBeginOverlap
  (params (OtherActor :type Actor%20Object%20Reference)))

(event EventTick
  (params (DeltaSeconds :type Float%20%28single-precision%29)))

(fn ConstructionScript)