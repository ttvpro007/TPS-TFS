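; CoverSlot is an actor, named as a cover position, that tracks which actors occupy it.
; Its Sphere's overlap events add and remove actors in CurrentOccupants.
; An enum State switches when an actor enters and reverts once no occupants remain.
; Each state assignment prints to screen, and entry also draws a brief debug sphere at the slot.
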(event OnComponentBeginOverlap(Sphere)
  (params (OverlappedComponent :type Primitive%20Component%20Object%20Reference) (OtherActor :type Actor%20Object%20Reference) (OtherComp :type Primitive%20Component%20Object%20Reference) (OtherBodyIndex :type Integer) (bFromSweep :type Boolean) (SweepResult :type Hit%20Result%20Structure%20%28by%20ref%29))
  (Utilities|Array|Add (Variables|Default|GetCurrentOccupants) OtherActor)
  (bind _output_get (Variables|Default|SetState "NewEnumerator1"))
  (Development|PrintString (Utilities|String|EnumtoString _output_get))
  (Rendering|Debug|DrawDebugSphere (Transformation|GetActorLocation) 1e+01 12 "(R=1.000000,G=1.000000,B=1.000000,A=1.000000)" 2.0))

(event OnComponentEndOverlap(Sphere)
  (params (OverlappedComponent :type Primitive%20Component%20Object%20Reference) (OtherActor :type Actor%20Object%20Reference) (OtherComp :type Primitive%20Component%20Object%20Reference) (OtherBodyIndex :type Integer))
  (bind _currentoccupants (Variables|Default|GetCurrentOccupants))
  (Utilities|Array|RemoveItem _currentoccupants OtherActor)
  (if (== (Utilities|Array|Length _currentoccupants) 0)
    (bind _output_get (Variables|Default|SetState "NewEnumerator0"))
    (Development|PrintString (Utilities|String|EnumtoString _output_get))))

(event EventBeginPlay)

(event Collision|EventActorBeginOverlap
  (params (OtherActor :type Actor%20Object%20Reference)))

(event EventTick
  (params (DeltaSeconds :type Float%20%28single-precision%29)))

(fn ConstructionScript)